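; Player pawn that detects touch swipes and spawns a ProjectileBall_BP at its XY position and a fixed height.
; Touch press and release record screen points; once pressed, Tick keeps checking their distance against a threshold, as the pressed flag never clears.
; A DoOnce, reset on release, samples Touch1, prints the dominant-axis direction and spawns the ball.
; One second later, all balls of that class are destroyed.
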(event Custom|Check_Swiping
  (bind _returnvalue (Game|GetPlayerController 0))
  (bind (_locationx _locationy) (Class|PlayerController|GetInputTouchState _returnvalue "Touch1"))
  (if (> (Math|Vector2D|Vector2DLength (- (Variables|Default|GetTouchStart) (Variables|Default|GetTouchEnd))) 1e+01)
    (Utilities|FlowControl|DoOnce false
      (:Completed
        (Variables|Default|SetTouchEnd (Math|Vector2D|MakeVector2D _locationx _locationy))
        (Variables|Default|SetOut%20Dir (.OutDir (Class|KismetMathLibrary|ToDirectionandLength2D (- (Variables|Default|GetTouchStart) (Variables|Default|GetTouchEnd)))))
        (Variables|Default|SetOut%20Length (.OutLength (Class|KismetMathLibrary|ToDirectionandLength2D (- (Variables|Default|GetTouchStart) (Variables|Default|GetTouchEnd)))))
        (if (> (Math|Float|Absolute(Float) (.X (Math|Vector2D|BreakVector2D (- (Variables|Default|GetTouchStart) (Variables|Default|GetTouchEnd))))) (Math|Float|Absolute(Float) (.Y (Math|Vector2D|BreakVector2D (- (Variables|Default|GetTouchStart) (Variables|Default|GetTouchEnd))))))
          (if (> (.X (Math|Vector2D|BreakVector2D (- (Variables|Default|GetTouchStart) (Variables|Default|GetTouchEnd)))) 0.0)
            (Development|PrintString "Left")
            (else
              (Development|PrintString "Right")))
          (elif (> (.Y (Math|Vector2D|BreakVector2D (- (Variables|Default|GetTouchStart) (Variables|Default|GetTouchEnd)))) 0.0)
            (Development|PrintString "Up")
            (else
              (Development|PrintString "Down"))))
        (CallFunction|SpawnBall)))))

(event Custom|Spawn_Ball
  (bind _defaultsceneroot (Variables|Default|GetDefaultSceneRoot))
  (bind _returnvalue (Transformation|GetWorldLocation _defaultsceneroot))
  (bind _returnvalue_2 (Game|SpawnActorfromClass "/Game/Nike_Game_Project/Blueprints/Pawn/ProjectileBall_BP.ProjectileBall_BP_C" (Math|Transform|MakeTransform (Math|Vector|MakeVector (.x _returnvalue) (.y _returnvalue) 1e+02) "0, 0, 0" "1,1,1") "Undefined" 0 0))
  (Utilities|FlowControl|Delay 1.0)
  (bind _outactors (Actor|GetAllActorsOfClass (Utilities|GetClass _returnvalue_2)))
  (Actor|DestroyActor _outactors))

(event EventTick
  (params (DeltaSeconds :type Float%20%28single-precision%29))
  (Utilities|FlowControl|Sequence
    (:then_0
      (Development|PrintString (Utilities|String|Append "Direction:  " (Utilities|String|ToString(Vector2d) (Variables|Default|GetOut%20Dir))) true true "(R=0.000000,G=0.004274,B=1.000000,A=1.000000)" 0.0)
      (Development|PrintString (Utilities|String|Append "Lenght:  " (Utilities|String|ToString(Float) (Variables|Default|GetOut%20Length))) true true "(R=0.000000,G=1.000000,B=0.102158,A=1.000000)" 0.0))
    (:then_1
      (if (Variables|Default|GetIsPressed)
        (CallFunction|CheckSwiping))
      (Development|PrintString (Utilities|String|Append "Screen Position: " (Utilities|String|ToString(Vector2d) (Variables|Default|GetTouchStart)) (Utilities|String|ToString(Vector2d) (Variables|Default|GetTouchEnd))) true true "(R=1.000000,G=0.000000,B=0.007303,A=1.000000)" 0.0))))

(event Input|TouchEvents|InputTouch
  (params (Location :type Vector) (FingerIndex :type ETouchIndex%20Enum))
  (bind (_x _y) (Math|Vector|BreakVector Location))
  (bind _returnvalue (Game|GetPlayerController 0))
  (bind (_locationx _locationy) (Class|PlayerController|GetInputTouchState _returnvalue "Touch1"))
  (:Pressed
    (Variables|Default|SetIsPressed true)
    (Variables|Default|SetTouchStart (Math|Vector2D|MakeVector2D _x _y)))
  (:Released
    (Variables|Default|SetTouchEnd (Math|Vector2D|MakeVector2D _x _y))
    (Utilities|FlowControl|DoOnce false) ; enters at Reset
  ))

(fn ConstructionScript)